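; BP_Soldier_01 is a player-controlled soldier with world-axis movement, mouse-driven facing and cosmetic rifle fire.
; Each tick, when mouse velocity exceeds MouseDeadZone, control rotation yaw interpolates toward the direction of mouse motion, not cursor position.
; Left mouse toggles the muzzle-flash effect and looping fire sound while held, playing an end-shot sound on release.
; No projectile, trace or damage logic is present.
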(event EventTick
  (params (DeltaSeconds :type Float%20%28single-precision%29))
  ;[1 1 1] Player Rotation
  (CallFunction|UpdatePlayerRotation))

(event Input|AxisEvents|InputAxisMoveBack
  (params (AxisValue :type Float%20%28single-precision%29))
  ;[1 1 1] Marine movements
  (Pawn|Input|AddMovementInput (Math|Vector|MakeVector AxisValue 0.0 0.0) 1.0 false))

(event Input|AxisEvents|InputAxisMoveLeftRight
  (params (AxisValue :type Float%20%28single-precision%29))
  ;[1 1 1] Marine movements
  (Pawn|Input|AddMovementInput (Math|Vector|MakeVector 0.0 AxisValue 0.0) 1.0 false))

(event Input|MouseEvents|LeftMouseButton
  (params (Key :type Key%20Structure :default "None"))
  ;[1 1 1] Effect Fire
  (:Pressed
    (CallFunction|ClickedtoFire))
  (:Released
    (CallFunction|StopFire)))

(fn ConstructionScript)

(fn UpdatePlayerRotation
  (bind _returnvalue (CallFunction|GetMouseVelocity))
  (bind _returnvalue_2 (Game|GetPlayerController 0))
  (if (CallFunction|IsMouseDeadZone)
    (Pawn|SetControlRotation _returnvalue_2 (Math|Interpolation|RInterpTo (Pawn|GetControlRotation _returnvalue_2 :!class /Script/Engine.Controller) (Math|Rotator|MakeRotator 0.0 0.0 (Class|KismetMathLibrary|DegAtan2 (.x _returnvalue) (.y _returnvalue))) (Utilities|Time|GetWorldDeltaSeconds) 7.0))))

(fn GetMouseVelocity
  (bind _returnvalue (Game|GetPlayerController 0))
  (bind (_deltax _deltay) (Class|PlayerController|GetInputMouseDelta _returnvalue))
  (return (/ (Math|Vector2D|MakeVector2D _deltax _deltay) (Utilities|Time|GetWorldDeltaSeconds))))

(fn IsMouseDeadZone
  (return (> (Math|Vector2D|Vector2DLength (CallFunction|GetMouseVelocity)) (Variables|Default|GetMouseDeadZone))))

(fn StopFire
  (Components|Activation|Deactivate (Variables|Default|GetP_AssaultRifle_MF))
  (Audio|Components|Audio|StopDelayed (Variables|Default|GetWeaponFireSound) 0.0)
  (Audio|SpawnSound2D "/Game/Sounds/Weapon_AssaultRifle/Stereo/AssaultRifle_EndShoot_Cue.AssaultRifle_EndShoot_Cue" 1.0 1.0 0.0 0))

(fn ClickedtoFire
  (Components|Activation|Activate (Variables|Default|GetP_AssaultRifle_MF) false)
  (bind _returnvalue (Audio|SpawnSound2D "/Game/Sounds/Weapon_AssaultRifle/Stereo/AssaultRifle_LoopShoot_Cue.AssaultRifle_LoopShoot_Cue" 1.0 1.0 0.0 0))
  (Variables|Default|SetWeaponFireSound _returnvalue))